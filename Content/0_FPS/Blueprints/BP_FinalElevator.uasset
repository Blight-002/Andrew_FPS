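; Final elevator actor in an FPS game that is held at the bottom until all cores have been collected.
; On BeginPlay it counts the BP_Core actors in the level and stores the total in Cores.
; While Cores is above zero, Tick resets the Cube to a fixed relative location every frame.
; Nothing in this graph decrements the count or raises the elevator.
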(event `self.ReceiveBeginPlay`
  (`parent.ReceiveBeginPlay`)
  ;[0.001073 0.4195 0.4896 0.5] Get Core Count
  (bind _outactors (`GameplayStatics.GetAllActorsOfClass` "/Game/0_FPS/Blueprints/BP_Core.BP_Core_C"))
  (set `self.Cores` (`KismetArrayLibrary.Array_Length` _outactors)))

(event `self.ReceiveTick`
  (params (DeltaSeconds :type "Float (single-precision)"))
  ;[0.5833 0.1733 0.1877 0.5] Keep at bottom if all cores havent been collected
  (if (> (`self.Cores`) 0)
    (`SceneComponent.K2_SetRelativeLocation` (`self.Cube`) (0.0 0.0 40.0) false false)))

(fn `UserConstructionScript`
  (`parent.UserConstructionScript`))