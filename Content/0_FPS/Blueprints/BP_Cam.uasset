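; BP_Cam is a security camera that makes the first-person player lose when it spots them.
; From BeginPlay, MoveCam loops itself, using a FlipFlop and MoveComponentTo to sweep the camera mesh between start and end rotations with a delay between moves.
; Every Tick, a debug-drawn Pawn object line trace runs forward from the LineTrace component.
; Hitting the cached player sets HasLost and disables their input.
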(event `MoveCam`
  ; Comment
  (`/Engine/EditorBlueprintResources/StandardMacros.FlipFlop`
    (:`A`
      (set `self.CurrentRotation` (`self.EndRotation`)))
    (:`B`
      (set `self.CurrentRotation` (`self.StartRotation`))))
  (`KismetSystemLibrary.MoveComponentTo` (`self.SM_Camera`) (0.0 0.0 0.0) (`self.CurrentRotation`) false false (`self.speed`))
  (`KismetSystemLibrary.Delay` (`self.Delay`))
  (`self.MoveCam`))

(event `self.ReceiveTick`
  (params (DeltaSeconds :type "Float (single-precision)"))
  (`self.Detect`))

(event `Detect`
  (bind _linetrace (`self.LineTrace`))
  (bind _player_reference (`self.Player Reference`))
  (bind _returnvalue (`SceneComponent.K2_GetComponentLocation` _linetrace))
  (bind _outhit (`KismetSystemLibrary.LineTraceSingleForObjects` :`Start` _returnvalue :`End` (+ _returnvalue (* (`KismetMathLibrary.GetForwardVector` (`SceneComponent.K2_GetComponentRotation` _linetrace)) (`self.DetectDistance`))) :`ObjectTypes` (`|MakeArray` "ObjectTypeQuery3" :!type "EObjectTypeQuery Enum") :`DrawDebugType` "ForOneFrame"))
  (if (== (`.HitActor` (`GameplayStatics.BreakHitResult` _outhit)) (`self.Player Reference`))
    (set `/Game/0_FPS/Blueprints/BP_FirstPersonCharacter.HasLost` true _player_reference)
    (`self.DisableInput` _player_reference (`GameplayStatics.GetPlayerController` 0))))

(event `self.ReceiveBeginPlay`
  (`|ExecutionSequence`
    (:`then_0`
      (bind _asbp_first_person_character (cast `/Game/0_FPS/Blueprints/BP_FirstPersonCharacter` (`GameplayStatics.GetPlayerCharacter` 0)))
      (set `self.Player Reference` _asbp_first_person_character))
    (:`then_1`
      (`self.MoveCam`))))

(fn `UserConstructionScript`)