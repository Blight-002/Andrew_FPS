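; Final elevator that rises while the player stands in its trigger, once its fuse count is down to zero.
; BeginPlay sets Fuses to the number of BP_Core actors in the level; nothing here decrements it.
; Overlap plays a timeline that lerps the Cube up to a Height-based Z, and leaving reverses it.
; TimeToTop scales the timeline's play rate to set travel speed.
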(event `self.ReceiveBeginPlay`
  ; Set Animation Speed
  (`TimelineComponent.SetPlayRate` (`self.Timeline`) (/ 30.0 (`self.TimeToTop`)))
  (bind _outactors (`GameplayStatics.GetAllActorsOfClass` "/Game/0_FPS/Blueprints/BP_Core.BP_Core_C"))
  (set `self.Fuses` (`KismetArrayLibrary.Array_Length` _outactors))
  (bind _asbp_first_person_character (cast `/Game/0_FPS/Blueprints/BP_FirstPersonCharacter` (`GameplayStatics.GetPlayerCharacter` 0)))
  (set `self.PlayerReference` _asbp_first_person_character))

(event `self.Collision.OnComponentBeginOverlap`
  (params (OverlappedComponent :type "PrimitiveComponent Object Reference") (OtherActor :type "Actor Object Reference") (OtherComp :type "PrimitiveComponent Object Reference") (OtherBodyIndex :type Integer) (bFromSweep :type Boolean) (SweepResult :type "HitResult Structure (by ref)"))
  (if (<= (`self.Fuses`) 0)
    (if (== OtherActor (`self.PlayerReference`))
      (bind (_direction _alpha) (`Timeline|Timeline` :!label _label)
        (:`Update`
          (`SceneComponent.K2_SetRelativeLocation` (`self.Cube`) (`KismetMathLibrary.VLerp` (0.0 0.0 40.0) (`KismetMathLibrary.MakeVector` 0.0 0.0 (* (`self.Height`) 1000.0)) _alpha) false false))))))

(event `self.Collision.OnComponentEndOverlap`
  (params (OverlappedComponent :type "PrimitiveComponent Object Reference") (OtherActor :type "Actor Object Reference") (OtherComp :type "PrimitiveComponent Object Reference") (OtherBodyIndex :type Integer))
  (if (<= (`self.Fuses`) 0)
    (if (== OtherActor (`self.PlayerReference`))
      (goto _label :!via `Reverse`))))

(fn `UserConstructionScript`
  (`parent.UserConstructionScript`))