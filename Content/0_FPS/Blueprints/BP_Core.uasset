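; BP_Core is a pickup core the player activates once by entering its sphere radius.
; On begin play it gives its mesh a dynamic blue light material and caches the player and the FinalElevator.
; On the first player overlap it turns dark red, decrements the elevator's remaining Cores count and refills the player's battery to maximum.
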(event `self.ReceiveBeginPlay`
  (`|ExecutionSequence`
    (:`then_0`
      (bind _returnvalue (`KismetMaterialLibrary.CreateDynamicMaterialInstance` "/Game/0_FPS/Materials/MI_Light_Blue.MI_Light_Blue"))
      (bind _output_get (set `self.CoreMaterial` _returnvalue))
      (`PrimitiveComponent.SetMaterial` (`self.Core`) 0 _output_get))
    (:`then_1`
      (bind _asbp_first_person_character (cast `/Game/0_FPS/Blueprints/BP_FirstPersonCharacter` (`GameplayStatics.GetPlayerCharacter` 0)))
      (set `self.PlayerReference` _asbp_first_person_character)
      (bind _returnvalue_2 (`GameplayStatics.GetActorOfClass` "/Game/0_FPS/Blueprints/FinalElevator.FinalElevator_C"))
      (set `self.ElevatorReference` _returnvalue_2))))

(event `self.Sphere.OnComponentBeginOverlap`
  (params (OverlappedComponent :type "PrimitiveComponent Object Reference") (OtherActor :type "Actor Object Reference") (OtherComp :type "PrimitiveComponent Object Reference") (OtherBodyIndex :type Integer) (bFromSweep :type Boolean) (SweepResult :type "HitResult Structure (by ref)"))
  (bind _playerreference (`self.PlayerReference`))
  ;[0.8698 0.8698 0.8698 0.5] First Time Player Enters Radius
  (if (and (== OtherActor (`self.PlayerReference`)) (`self.FirstHit`))
    ;;[0 0.4804 0.5312 0.5] Change colour
    (`MaterialInstanceDynamic.SetVectorParameterValue` (`self.CoreMaterial`) "Colour" (struct :`R` 0.075 :`A` 1.0))
    ;;[0.4435 0 0 0.5] Reduce From Core Count
    (`/Engine/EditorBlueprintResources/StandardMacros.DecrementInt` (`/Game/0_FPS/Blueprints/FinalElevator.Cores` (`self.ElevatorReference`))
      (:`  `
        ;;[0 1 0 0.5] Recharge Battery
        (set `/Game/0_FPS/Blueprints/BP_FirstPersonCharacter.CurrentBattery` (`/Game/0_FPS/Blueprints/BP_FirstPersonCharacter.MaxBattery` _playerreference) _playerreference)
        (set `self.FirstHit` false)))))

(fn `UserConstructionScript`)