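; Key-locked door for an FPS game that swings open when the player enters its trigger while holding a key, with an indicator light showing access.
; On BeginPlay it caches the player character and gives the light mesh a dynamic material instance.
; Trigger overlap brightens the light green or red depending on HasKey; leaving dims it to yellow.
; A timeline lerps the door's rotation, reversing on exit, and maintains a DoorOpening flag.
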(event `self.ReceiveBeginPlay`
  ; setup variables
  (`|ExecutionSequence`
    (:`then_0`
      (bind _asbp_first_person_character (cast `/Game/0_FPS/Blueprints/BP_FirstPersonCharacter` (`GameplayStatics.GetPlayerCharacter` 0)))
      (set `self.Player Reference` _asbp_first_person_character))
    (:`then_1`
      (bind _returnvalue (`KismetMaterialLibrary.CreateDynamicMaterialInstance` "/Game/0_FPS/Materials/MI_Light.MI_Light"))
      (bind _output_get (set `self.DynamicMateral` _returnvalue))
      (`PrimitiveComponent.SetMaterial` (`self.SM_Light`) 0 _output_get))))

(event `self.Trigger.OnComponentBeginOverlap`
  (params (OverlappedComponent :type "PrimitiveComponent Object Reference") (OtherActor :type "Actor Object Reference") (OtherComp :type "PrimitiveComponent Object Reference") (OtherBodyIndex :type Integer) (bFromSweep :type Boolean) (SweepResult :type "HitResult Structure (by ref)"))
  ; Light CHange
  (if (== OtherActor (`self.Player Reference`))
    (`MaterialInstanceDynamic.SetScalarParameterValue` (`self.DynamicMateral`) "Brightness" 1.0)
    (if (`/Game/0_FPS/Blueprints/BP_FirstPersonCharacter.hasKey` (`self.Player Reference`))
      (`MaterialInstanceDynamic.SetVectorParameterValue` (`self.DynamicMateral`) "Colour" (struct :`G` 1.0 :`A` 1.0))
      ; Door OpenClose
      (bind (_direction _alpha) (`Timeline|Timeline_DoorOpenClose` :!label _label)
        (:`Update`
          (set `self.Door Opening` true)
          (`SceneComponent.K2_SetRelativeRotation` (`self.SM_Door`) (`KismetMathLibrary.RLerp` (struct) (struct :`Yaw` 90.0) _alpha) false false))
        (:`Finished`
          (set `self.Door Opening` false)))
      (else
        (`MaterialInstanceDynamic.SetVectorParameterValue` (`self.DynamicMateral`) "Colour" (struct :`R` 1.0 :`A` 1.0))))))

(event `self.Trigger.OnComponentEndOverlap`
  (params (OverlappedComponent :type "PrimitiveComponent Object Reference") (OtherActor :type "Actor Object Reference") (OtherComp :type "PrimitiveComponent Object Reference") (OtherBodyIndex :type Integer))
  (bind _dynamicmateral (`self.DynamicMateral`))
  (if (== OtherActor (`self.Player Reference`))
    (`MaterialInstanceDynamic.SetScalarParameterValue` _dynamicmateral "Brightness" 0.01)
    (`MaterialInstanceDynamic.SetVectorParameterValue` _dynamicmateral "Colour" (struct :`R` 1.0 :`G` 0.983486 :`B` 0.175769 :`A` 1.0))
    (goto _label :!via `Reverse`)))

(fn `UserConstructionScript`)