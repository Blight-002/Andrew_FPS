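; BP_Elevator is a platform that rises while the first-person player is in its collision volume and descends when they leave.
; BeginPlay caches the player character and sets the rise timeline's play rate from TimeToTop, so travel time is configurable.
; Overlap begin plays the timeline and overlap end reverses it, interpolating the cube's relative location between a fixed base offset and a height scaled from the Height variable.
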(event `self.ReceiveBeginPlay`
  ;[0.01626 0.05841 0.15 0.5] Player Reference
  (bind _asbp_first_person_character (cast `/Game/0_FPS/Blueprints/BP_FirstPersonCharacter` (`GameplayStatics.GetPlayerCharacter` 0)))
  (set `self.PlayerReference` _asbp_first_person_character)
  ;[0.0233 0.8494 1 0.5] Set Animation Speed
  (`TimelineComponent.SetPlayRate` (`self.TimeLine_Rise`) (/ 1.0 (`self.TimeToTop`))))

(event `self.Collision.OnComponentBeginOverlap`
  (params (OverlappedComponent :type "PrimitiveComponent Object Reference") (OtherActor :type "Actor Object Reference") (OtherComp :type "PrimitiveComponent Object Reference") (OtherBodyIndex :type Integer) (bFromSweep :type Boolean) (SweepResult :type "HitResult Structure (by ref)"))
  ;[0.527 0.7031 0.015 0.5] Elevator Rise and Fall
  (if (== OtherActor (`self.PlayerReference`))
    (bind (_direction _alpha) (`Timeline|TimeLine_Rise` :!label _label)
      (:`Update`
        (`SceneComponent.K2_SetRelativeLocation` (`self.Cube`) (`KismetMathLibrary.VLerp` (0.0 0.0 40.0) (`KismetMathLibrary.MakeVector` 0.0 0.0 (* (`self.Height`) 1000.0)) _alpha) false false)))))

(event `self.Collision.OnComponentEndOverlap`
  (params (OverlappedComponent :type "PrimitiveComponent Object Reference") (OtherActor :type "Actor Object Reference") (OtherComp :type "PrimitiveComponent Object Reference") (OtherBodyIndex :type Integer))
  ;[0.527 0.7031 0.015 0.5] Elevator Rise and Fall
  (if (== OtherActor (`self.PlayerReference`))
    (goto _label :!via `Reverse`)))

(fn `UserConstructionScript`)