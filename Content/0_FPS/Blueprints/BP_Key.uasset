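; BP_Key is a collectible key that appears once no BP_Target actors remain in the level.
; Each tick it counts the targets and toggles its visibility and collision, playing an appear sound and particle effect once when the count hits zero.
; When the player's capsule overlap is detected, it sets HasKey on the first-person character, plays a collect sound and destroys itself.
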(event `self.ReceiveBeginPlay`
  ; Set up variables
  (bind _asbp_first_person_character (cast `/Game/0_FPS/Blueprints/BP_FirstPersonCharacter` (`GameplayStatics.GetPlayerCharacter` 0)))
  (set `self.Player Reference` _asbp_first_person_character))

(event `self.ReceiveTick`
  (params (DeltaSeconds :type "Float (single-precision)"))
  (bind _returnvalue (`SceneComponent.K2_GetComponentLocation` (`self.DefaultSceneRoot`)))
  ; Key Visability
  (bind _outactors (`GameplayStatics.GetAllActorsOfClass` "/Game/0_FPS/Blueprints/BP_Target.BP_Target_C"))
  (`|ExecutionSequence`
    (:`then_0`
      (bind _returnvalue_2 (== (`KismetArrayLibrary.Array_Length` _outactors) 0))
      (`SceneComponent.SetVisibility` (`self.DefaultSceneRoot`) _returnvalue_2 true)
      (`self.SetActorEnableCollision` _returnvalue_2)
      ; Key Appear
      (if _returnvalue_2
        (`/Engine/EditorBlueprintResources/StandardMacros.DoOnce` false
          (:`Completed`
            (`GameplayStatics.PlaySoundAtLocation` "/Game/0_FPS/Audio/MP3_Key_Appear.MP3_Key_Appear" _returnvalue (struct) 1.0 1.0 0.0 null null null null)
            (`GameplayStatics.SpawnEmitterAtLocation` "/Engine/Tutorial/SubEditors/TutorialAssets/TutorialParticleSystem.TutorialParticleSystem" _returnvalue)))))))

(event `self.Capsule.OnComponentBeginOverlap`
  (params (OverlappedComponent :type "PrimitiveComponent Object Reference") (OtherActor :type "Actor Object Reference") (OtherComp :type "PrimitiveComponent Object Reference") (OtherBodyIndex :type Integer) (bFromSweep :type Boolean) (SweepResult :type "HitResult Structure (by ref)"))
  ; Key Pickup
  (if (== OtherActor (`self.Player Reference`))
    (set `/Game/0_FPS/Blueprints/BP_FirstPersonCharacter.hasKey` true (`self.Player Reference`))
    (`GameplayStatics.PlaySoundAtLocation` "/Game/0_FPS/Audio/MP3_Key_Collect.MP3_Key_Collect" (`self.K2_GetActorLocation`) (struct) 1.0 1.0 0.0 null null null null)
    (`self.K2_DestroyActor`)))

(fn `UserConstructionScript`)